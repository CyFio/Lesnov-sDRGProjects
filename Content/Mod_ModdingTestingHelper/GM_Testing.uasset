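; A testing game mode for a modding helper that runs an endless enemy-spawn score session.
; After level generation it starts the game, creates a score widget, and waits for the local player to enter and then leave the drop pod.
; It then starts a looping timer that spawns random enemies around a point, while kill events add points to the widget.
; Unwired experiments for resupply pods and loadout swapping remain in the graphs.
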(event Custom|CustomEvent_2
  (params (enemyTags :type Gameplay%20Tag%20Container%20Structure%20%28by%20ref%29) (enemy :type Actor%20Object%20Reference) (DamageClass :type Damage%20Class%20Object%20Reference))
  (bind _point (Variables|Default|GetPoint))
  (Utilities|IsValid (Variables|Default|GetNewVar_0)
    (:Is%20Valid
      (|SetBy-RefVar _point (+ _point 50))
      (Default|SetScore (Variables|Default|GetNewVar_0) (Variables|Default|GetPoint)))))

(event Custom|OnGameStarted
  (|CollapseGraph_0))

(event EventBeginPlay
  (|CallParentFunction) ; This node is disabled and will not be called.\nDrag off pins to build functionality.
)

(event EventTick
  (params (DeltaSeconds :type Float%20%28single-precision%29))
  (|CallParentFunction DeltaSeconds) ; This node is disabled and will not be called.\nDrag off pins to build functionality.
)

(event EventOnLevelGenerationComplete
  (params (pass :type Integer))
  (|CallParentFunction pass)
  (Class|FSDGameMode|StartGame)
  (Utilities|FlowControl|Sequence
    (:then_0
      (Utilities|FlowControl|DoOnce false
        (:Completed
          (bind _fsdplayercontroller (Utilities|GetLocalPlayerController(Macro) true)
            (:Completed
              (Variables|Default|SetFSDPlayer%20Controller _fsdplayercontroller)
              (bind _playercharacter (Utilities|GetLocalPlayerCharacter(Macro) true)
                (:Exec
                  (bind _output_get (Variables|Default|SetPlayer%20Character _playercharacter))
                  (EventDispatchers|BindEventtoOnEnemyKilledEvent (Class|PlayerCharacter|GetPlayerState _output_get) (delegate Custom|CustomEvent_2))
                  (bind _outputpin (Utilities|WaitUntil(CreateWidge) "/Game/_DRGModding/Mod_ModdingTestingHelper/Widget.Widget_C" (Variables|Default|GetFSDPlayer%20Controller))
                    (:true
                      (bind _aswidget (Utilities|Casting|CastToWidget _outputpin))
                      (Variables|Default|SetNewVar_0 _aswidget)
                      (Utilities|WaitUntilTrue (Variables|/Script/FSD.PlayerCharacter|GetIsInDropPod (Variables|Default|GetPlayer%20Character))
                        (:true
                          (Utilities|WaitUntilTrue (not (Variables|/Script/FSD.PlayerCharacter|GetIsInDropPod (Variables|Default|GetPlayer%20Character)))
                            (:true
                              (CallFunction|OnGameStarted))))))))))))))))

(fn ConstructionScript
  (|CallParentFunction))

(event Custom|CustomEvent_0
  (Class|EnemySpawnManager|SpawnEnemy (Variables|Default|GetEnemySpawnManager) (.OutItem (Utilities|Array|Random (Variables|Default|GetDescriptor))) (Math|Transform|MakeTransform (Class|SpawningBlueprintLibrary|GetSpawnPointfromLocation self "0, 0, 0" 3e+03 "Large") "0, 0, 0" "1,1,1") (delegate Custom|CustomEvent_1) false true))

(event Custom|CustomEvent_1
  (params (enemy :type Pawn%20Object%20Reference)))