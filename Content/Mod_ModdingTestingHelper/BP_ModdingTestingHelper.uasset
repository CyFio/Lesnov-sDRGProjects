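; Testing helper actor for Deep Rock Galactic modding that adds chat-driven debug commands and a persistent custom spawn point.
; BeginPlay retries loading MTHSavegame, resolves the local controller and character, then moves the player to the saved spawn when not in a cave.
; Chat messages pass through a sender filter into a string switch for saving spawn, quick-starting a solo mission, returning to the space rig, and player-count and inventory tweaks.
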(event EventBeginPlay
  (bind _outputpin (Utilities|HandleSaveGame "/Game/_DRGModding/Mod_ModdingTestingHelper/MTHSavegame.MTHSavegame_C" :!label _label)
    (:then
      (bind _asmthsavegame (Utilities|Casting|CastToMTHSavegame _outputpin))
      (Variables|Default|SetAs%20MTHSavegame _asmthsavegame)
      (bind _fsdplayercontroller (Utilities|GetLocalPlayerController(Macro) true)
        (:Completed
          (Variables|Default|SetFSDPlayer%20Controller _fsdplayercontroller)
          (bind _playercharacter (Utilities|GetLocalPlayerCharacter(Macro) true)
            (:Exec
              (Variables|Default|SetPlayer%20Character _playercharacter)
              (|QuickConsoleCommand(TFPS)_2) ; Used to implement console command quickly via chat
              (if (not (Variables|Default|GetIsInCave))
                (bind (_newspawnpoint _returnvalue) (Default|GetNewSpawnLocation (Variables|Default|GetAs%20MTHSavegame)))
                (if _returnvalue
                  (Transformation|SetActorTransform (Variables|Default|GetPlayer%20Character) (Math|Transform|MakeTransform (.Location (Math|Transform|BreakTransform _newspawnpoint)) "0, 0, 0" (Transformation|GetActorScale3D (Variables|Default|GetPlayer%20Character))))
                  (Pawn|SetControlRotation (Variables|Default|GetFSDPlayer%20Controller) (.Rotation (Math|Transform|BreakTransform _newspawnpoint))))))))))
    (:ERROR
      (Utilities|FlowControl|Delay 0.2)
      (goto _label))))

(event EventTick
  (params (DeltaSeconds :type Float%20%28single-precision%29)))

(fn ConstructionScript)

(fn Save
  (Utilities|SavetoSlot(Macro) (Variables|Default|GetAs%20MTHSavegame)))

(event Custom|OnNewMessage
  (params (Message :type FSD%20Chat%20Message%20Structure%20%28by%20ref%29))
  (bind _msg (Utilities|IgnoreMsgbySender Message (Variables|Default|GetPlayer%20Character))
    (:CanProceed
      (|Outputs _msg) ; enters at OnReceiveChat
    )))