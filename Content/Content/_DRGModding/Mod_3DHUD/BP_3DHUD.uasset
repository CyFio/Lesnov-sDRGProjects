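; Deep Rock Galactic "3D HUD" mod actor that attaches a world-space HUD to the first-person camera, with input-driven sway.
; BeginPlay loads saved color, then binds health, armor, inventory, Bosco and shoulder-weapon events to the widget, with throttled alert sounds.
; Tick traces for range and target health, and predicts projectile impacts to place a marker.
; A timer counts nearby enemies, and a chat command toggles transform-tuning sliders.
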(event Custom|CustomEvent_0
  (params (Vector :type Vector))
  (Transformation|SetActorRelativeLocation (* Vector 2e+01)))

(event Custom|CustomEvent_1
  (params (Vector :type Vector))
  (Transformation|SetActorRelativeRotation (Math|Conversions|RotationFromXVector Vector)))

(event Custom|CustomEvent_5
  (CallFunction|NewFunction1))

(event Custom|CustomEvent_6
  (Variables|Default|SetCanSound_ShieldEmpty true))

(event Custom|OnColorChanged_Event_0
  (params (LinearColor :type Linear%20Color%20Structure))
  (CallFunction|SetHUDColor LinearColor)
  (Variables|/Game/_DRGModding/Mod_3DHUD/3DHUDSaveGame.3DHUDSaveGame_C|SetHUDColor (Variables|Default|GetAs%203DHUDSave%20Game) LinearColor)
  (Utilities|SavetoSlot(Macro) (Variables|Default|GetAs%203DHUDSave%20Game)))

(event Custom|ss
  (Variables|Default|SetCanSound_Health true))

(event Custom|OnHealthChanged_Event_0
  (params (Health :type Float%20%28single-precision%29))
  (bind _player_character (Variables|Default|GetPlayer%20Character))
  (bind _healthcomponent (Variables|/Script/FSD.PlayerCharacter|GetHealthComponent _player_character))
  (bind _maxhealth (Variables|/Script/FSD.PlayerHealthComponent|GetMaxHealth _healthcomponent))
  (bind _returnvalue (/ Health _maxhealth))
  (Default|SetHealth (Variables|Default|GetAs%20MENU%20HUDTesting) _returnvalue)
  (if (< _returnvalue 0.2)
    (if (Variables|Default|GetCanSound_Health)
      (bind _isplayed (CallFunction|PlaySound (Variables|Default|GetSound)))
      (if _isplayed
        (Variables|Default|SetCanSound_Health false)
        (Utilities|Time|SetTimerbyEvent (delegate Custom|ss) 1e+01)))))

(event Custom|OnArmorChanged_Event_0
  (params (Health :type Float%20%28single-precision%29))
  (bind _player_character (Variables|Default|GetPlayer%20Character))
  (bind _healthcomponent (Variables|/Script/FSD.PlayerCharacter|GetHealthComponent _player_character))
  (bind _maxarmor (Variables|/Script/FSD.PlayerHealthComponent|GetMaxArmor _healthcomponent))
  (bind _returnvalue (/ Health _maxarmor))
  (Default|SetArmor (Variables|Default|GetAs%20MENU%20HUDTesting) _returnvalue)
  (if (== _returnvalue 0.0)
    (if (Variables|Default|GetCanSound_ShieldEmpty)
      (bind _isplayed (CallFunction|PlaySound (Variables|Default|GetSound_0)))
      (if _isplayed
        (Variables|Default|SetCanSound_ShieldEmpty false)
        (Utilities|Time|SetTimerbyEvent (delegate Custom|CustomEvent_6) 1e+01)))
    (elif (== _returnvalue 1.0)
      (if (Variables|Default|GetCanSound_ShieldFull)
        (bind _isplayed_2 (CallFunction|PlaySound (Variables|Default|GetSound_1)))
        (if _isplayed_2
          (Variables|Default|SetCanSound_ShieldFull false)
          (Utilities|Time|SetTimerbyEvent (delegate Custom|dwadaw) 1.0))))))

(event Custom|OnPlayerHit_Event_0
  (params (Damage :type Float%20%28single-precision%29) (DamageData :type Damage%20Data%20Structure%20%28by%20ref%29) (anyHealthLost :type Boolean))
  (Default|OnHit (Variables|/Game/_DRGModding/Mod_3DHUD/MENU_HUDTesting.MENU_HUDTesting_C|GetHUD_Directional_Damage_IndicatorV2 (Variables|Default|GetAs%20MENU%20HUDTesting)) Damage DamageData anyHealthLost))

(event Custom|test
  (if (Variables|Default|GetCanSound_ShieldEmpty)
    (bind _isplayed (CallFunction|PlaySound (Variables|Default|GetSound_0)))
    (if _isplayed
      (Variables|Default|SetCanSound_ShieldEmpty false)
      (Utilities|Time|SetTimerbyEvent (delegate Custom|CustomEvent_6) 1e+01))))

(event Custom|dwadaw
  (Variables|Default|SetCanSound_ShieldFull true))

(event Custom|OnTargetChanged_Event_0
  (params (NewTarget :type Actor%20Object%20Reference) (NewPrimitive :type Primitive%20Component%20Object%20Reference)))

(event EventBeginPlay
  (bind _returnvalue (UserInterface|CreateWidget "/Game/_DRGModding/Mod_3DHUD/HUBMENU_3DHUD.HUBMENU_3DHUD_C" :!label _label))
  (Utilities|IsValid _returnvalue
    (:Is%20Valid
      (Variables|Default|SetHUBMENU _returnvalue)
      (bind _outputpin (Utilities|HandleSaveGame "/Game/_DRGModding/Mod_3DHUD/3DHUDSaveGame.3DHUDSaveGame_C" :!label _label_2)
        (:then
          (bind _as3dhudsave_game (Utilities|Casting|CastTo3DHUDSaveGame _outputpin))
          (Variables|Default|SetAs%203DHUDSave%20Game _as3dhudsave_game)
          (bind _asmenu_hudtesting (Utilities|Casting|CastToMENU_HUDTesting (UserInterface|GetWidget (Variables|Default|GetWidget))))
          (Variables|Default|SetAs%20MENU%20HUDTesting _asmenu_hudtesting)
          (CallFunction|SetHUDColor (Variables|/Game/_DRGModding/Mod_3DHUD/3DHUDSaveGame.3DHUDSaveGame_C|GetHUDColor (Variables|Default|GetAs%203DHUDSave%20Game)))
          (Default|Initialize (Variables|Default|GetHUBMENU) (Variables|/Game/_DRGModding/Mod_3DHUD/3DHUDSaveGame.3DHUDSaveGame_C|GetHUDColor (Variables|Default|GetAs%203DHUDSave%20Game)))
          (EventDispatchers|AssignOnColorChanged (Variables|Default|GetHUBMENU) (delegate Custom|OnColorChanged_Event_0))
          (Collision|SetActorEnableCollision false)
          (bind _fsdplayercontroller (Utilities|GetLocalPlayerController(Macro) true)
            (:Completed
              (Input|EnableInput _fsdplayercontroller)
              (Utilities|IsinDRG
                (:In%20DRG
                  _)
                (:In%20Editor
                  (bind _returnvalue_2 (Game|SpawnActorfromClass "/Game/_DRGModding/Mod_3DHUD/EditorInput_3DHUD.EditorInput_3DHUD_C" (Math|Transform|MakeTransform "0, 0, 0" "0, 0, 0" "1,1,1") "AlwaysSpawn" 0 0))
                  (Variables|Default|SetNewVar_0 _returnvalue_2)))
              (bind _playercharacter (Utilities|GetLocalPlayerCharacter(Macro) true)
                (:Exec
                  (bind _output_get (Variables|Default|SetPlayer%20Character _playercharacter))
                  (Utilities|WaitUntilValid(Inventory-Items|EditorSkip) _output_get
                    (:Found
                      (|CollapseGraph_0)
                      (|InitializeBoscoHud
                        (:OutputPin
                          (bind _returnvalue_3 (Game|SpawnActorfromClass "/Game/_DRGModding/Mod_3DHUD/BP_ProjectilePredictMarker.BP_ProjectilePredictMarker_C" (Math|Transform|MakeTransform "0, 0, 0" "0, 0, 0" "1,1,1") "AlwaysSpawn" 0 0))
                          (Variables|Default|SetPredictMarker _returnvalue_3)
                          (EventDispatchers|AssignOnHealthChanged (Variables|/Script/FSD.PlayerCharacter|GetHealthComponent (Variables|Default|GetPlayer%20Character)) (delegate Custom|OnHealthChanged_Event_0))
                          (EventDispatchers|AssignOnArmorChanged (Variables|/Script/FSD.PlayerCharacter|GetHealthComponent (Variables|Default|GetPlayer%20Character)) (delegate Custom|OnArmorChanged_Event_0))
                          (Variables|Default|SetRelative%20Rotation (Variables|/Script/Engine.SceneComponent|GetRelativeRotation (Variables|Default|GetWidget)))
                          (EventDispatchers|AssignOnPlayerHit (Variables|/Script/FSD.PlayerCharacter|GetHealthComponent (Variables|Default|GetPlayer%20Character)) (delegate Custom|OnPlayerHit_Event_0))
                          (Utilities|IsValid (Variables|Default|GetNewVar_0)
                            (:Is%20Valid
                              (Variables|/Game/_DRGModding/Mod_3DHUD/EditorInput_3DHUD.EditorInput_3DHUD_C|SetAs%20MENU%20HUDTesting (Variables|Default|GetNewVar_0) (Variables|Default|GetAs%20MENU%20HUDTesting)))
                            (:Is%20Not%20Valid
                              _))
                          (Default|SetGrenade (Variables|Default|GetAs%20MENU%20HUDTesting) (select (Class|KismetSystemLibrary|IsPackagedforDistribution) (Variables|/Script/FSD.ThrownGrenadeItem|GetMaxGrenades (Variables|/Script/FSD.InventoryComponent|GetGrenadeItem (Variables|/Script/FSD.PlayerCharacter|GetInventoryComponent (Variables|Default|GetPlayer%20Character)))) 4))
                          (Default|SetFlare (Variables|Default|GetAs%20MENU%20HUDTesting) (select (Class|KismetSystemLibrary|IsPackagedforDistribution) (Variables|/Script/FSD.InventoryComponent|GetMaxFlares (Variables|/Script/FSD.PlayerCharacter|GetInventoryComponent (Variables|Default|GetPlayer%20Character))) 4))
                          (|ShoulderWeaponSystem)
                          (Transformation|AttachComponentToComponent (Variables|/Script/FSD.PlayerCharacter|GetFirstPersonCamera (Variables|Default|GetPlayer%20Character)) "" "SnapToTarget" "SnapToTarget" "KeepWorld" true)
                          (Transformation|SetActorRelativeLocation "800.000000, 0, 0")
                          (Utilities|IsinDRG
                            (:In%20DRG
                              (Transformation|SetActorRelativeRotation (Math|Conversions|RotationFromXVector "-0.100000, 0, 0")))
                            (:In%20Editor
                              (Transformation|SetActorRelativeRotation (Math|Conversions|RotationFromXVector "0.000000,5.621521, 0"))))
                          (Default|Initialize (Variables|Default|GetAs%20MENU%20HUDTesting) (Variables|Default|GetPlayer%20Character))
                          (Utilities|FlowControl|Sequence
                            (:then_0
                              (Utilities|Time|SetTimerbyEvent (delegate Custom|CustomEvent_5) 5.0 true)
                              (CallFunction|NewFunction1))
                            (:then_1
                              (|QuickConsoleCommand(TFPS)_2_2_2) ; Used to implement console command quickly via chat
                              (Utilities|FlowControl|Delay 4.0)
                              (CallFunction|PlaySound (Variables|Default|GetSoundStartUp)))))))))))))
        (:ERROR
          (Utilities|FlowControl|Delay 0.5)
          (goto _label_2))))
    (:Is%20Not%20Valid
      (Utilities|FlowControl|Delay 0.5)
      (goto _label))))

(event Collision|EventActorBeginOverlap
  (params (OtherActor :type Actor%20Object%20Reference)))

(event EventTick
  (params (DeltaSeconds :type Float%20%28single-precision%29))
  (bind _returnvalue (Class|Actor|GetInputAxisKeyValue))
  (bind _player_character (Variables|Default|GetPlayer%20Character))
  (bind _as_menu_hudtesting (Variables|Default|GetAs%20MENU%20HUDTesting))
  (bind _player_character_2 (Variables|Default|GetPlayer%20Character))
  (bind _firstpersoncamera (Variables|/Script/FSD.PlayerCharacter|GetFirstPersonCamera _player_character))
  (bind _ui_enemyhealthbar (Variables|/Game/_DRGModding/Mod_3DHUD/MENU_HUDTesting.MENU_HUDTesting_C|GetUI_EnemyHealthBar _as_menu_hudtesting))
  (bind _sightcomponent (Variables|/Script/FSD.PlayerCharacter|GetSightComponent _player_character_2))
  (bind (_start _end) (Utilities|GetLinetracePos _firstpersoncamera 10000))
  (bind _targethealth (Variables|/Script/FSD.CharacterSightComponent|GetTargetHealth _sightcomponent))
  (bind _returnvalue_2 (Class|Health|GetHealth _targethealth))
  (bind _returnvalue_3 (Class|Health|GetMaxHealth _targethealth))
  (Transformation|SetRelativeRotation (Variables|Default|GetWidget) (Math|Rotator|CombineRotators (Variables|Default|GetRelative%20Rotation) (Math|Rotator|MakeRotator (* _returnvalue 0.2) (Class|Actor|GetInputAxisKeyValue) (* _returnvalue 0.8))) false false)
  (|CollapseGraph_2)
  (Utilities|IsValid _player_character
    (:Is%20Valid
      (Variables|Default|SetStart _start)
      (bind (_outhit _returnvalue_4) (Collision|LineTraceByChannel _start _end "TraceTypeQuery3" false (Utilities|Array|MakeArray _player_character) "None"))
      (if _returnvalue_4
        (CallFunction|NewFunction0 (Variables|/Game/_DRGModding/Mod_3DHUD/MENU_HUDTesting.MENU_HUDTesting_C|Gettest (Variables|Default|GetAs%20MENU%20HUDTesting)) (.Location (Collision|BreakHitResult _outhit)))
        (Utilities|IsinDRG
          (:In%20DRG
            (if (> _returnvalue_2 0.0)
              (Default|SetHealthBar _ui_enemyhealthbar (Math|Float|SafeDivide _returnvalue_2 _returnvalue_3))
              (Default|SetHealthText _ui_enemyhealthbar (Math|Float|Truncate _returnvalue_2) (Math|Float|Truncate _returnvalue_3))
              (else
                (Default|SetHealthBar (Variables|/Game/_DRGModding/Mod_3DHUD/MENU_HUDTesting.MENU_HUDTesting_C|GetUI_EnemyHealthBar (Variables|Default|GetAs%20MENU%20HUDTesting)) 0.0)
                (Default|ToggleCrosshair (Variables|Default|GetAs%20MENU%20HUDTesting) false)))))))))

(fn ConstructionScript)

(fn NewFunction0
  (params (self2 :type Test%20Object%20Reference) (V2 :type Vector))
  (Default|SetText self2 (Utilities|Text|ToText(String) (Utilities|String|ToString(Integer) (Math|Float|Truncate (/ (Math|Vector|Distance(Vector) (Variables|Default|GetStart) V2) 1e+02))))))

(fn NewFunction1
  (bind _as_menu_hudtesting (Variables|Default|GetAs%20MENU%20HUDTesting))
  (bind _outactors (Collision|SphereOverlapActors (Transformation|GetActorLocation (Variables|Default|GetPlayer%20Character)) 3e+03 (Utilities|Array|MakeArray "ObjectTypeQuery9") "/Script/FSD.EnemyDeepPathfinderCharacter"))
  (bind _output_get (LocalVariables|SetNewLocalVar_0 (Utilities|Array|Length _outactors)))
  (CallFunction|DebugMessage (Utilities|String|ToString(Integer) _output_get))
  (for _array_element _outactors
    (if (Utilities|ClassIsChildOf (Utilities|GetClass _array_element) "/Script/FSD.AFlyingBug")
      (Math|Integer|IncrementInt (LocalVariables|GetNewLocalVar_1))))
  (Default|SetText (Variables|/Game/_DRGModding/Mod_3DHUD/MENU_HUDTesting.MENU_HUDTesting_C|Gettest_1 _as_menu_hudtesting) (Utilities|Text|ToText(Integer) (LocalVariables|GetNewLocalVar_1)))
  (Default|SetText (Variables|/Game/_DRGModding/Mod_3DHUD/MENU_HUDTesting.MENU_HUDTesting_C|Gettest_2 _as_menu_hudtesting) (Utilities|Text|ToText(Integer) (LocalVariables|GetNewLocalVar_0))))

(fn DebugMessage
  (params (Sender :type String) (Text :type String))
  (Utilities|PrintViaChat (Variables|Default|GetDisable%20Debug) (Utilities|QuickAppend(Macro) "3DHUD" Sender) Text "NormalUser"))

(fn PlaySound
  (params (Sound :type Sound%20Cue%20Object%20Reference))
  (Utilities|IsValid (Variables|Default|GetNewVar_1)
    (:Is%20Valid
      (if (not (Audio|Components|Audio|IsPlaying (Variables|Default|GetNewVar_1)))
        (bind _returnvalue (Audio|SpawnSound2D Sound 1.0 1.0 0.0 0 :!label _label))
        (Variables|Default|SetNewVar_1 _returnvalue)
        (return true)))
    (:Is%20Not%20Valid
      (goto _label))))

(fn SetBoscoRocketCount
  (params (Value :type Integer))
  (Default|InitializeSubText (Variables|/Game/_DRGModding/Mod_3DHUD/MENU_HUDTesting.MENU_HUDTesting_C|GetCUI_BoscoInfos (Variables|Default|GetAs%20MENU%20HUDTesting)) (Utilities|Text|ToText(Integer) Value) (Utilities|Text|ToText(Integer) (Class|BoscoAbillityComponent|GetMaxCharges (Class|Bosco|GetPlayerAbillity (Variables|Default|GetAs%20BP%20Bosco))))))

(fn SetHUDColor
  (params (InColorAndOpacity :type Linear%20Color%20Structure))
  (Appearance|SetColorandOpacity (Variables|Default|GetAs%20MENU%20HUDTesting) InColorAndOpacity :!class /Script/UMG.UserWidget))

(fn HasValidProjectile
  (params (self2 :type Actor%20Object%20Reference))
  (bind _returnvalue (Actor|GetComponentbyClass self2 "/Script/FSD.ProjectileLauncherComponent"))
  (bind _asanimated_item (Utilities|Casting|CastToAnimatedItem self2)
    (:then
      (Variables|Default|SetAs%20Animated%20Item _asanimated_item)
      (Utilities|IsValid _returnvalue
        (:Is%20Valid
          (bind _asprojectile (Utilities|Casting|CastToProjectileClass (Variables|/Script/FSD.ProjectileLauncherComponent|GetProjectileClass _returnvalue))
            (:then
              (bind _returnvalue_2 (Class|ActorFunctionLibrary|GetComponentfromClass _asprojectile "/Script/Engine.ProjectileMovementComponent"))
              (bind _asprojectile_movement_component (Utilities|Casting|CastToProjectileMovementComponent _returnvalue_2)
                (:then
                  (bind _output_get (Variables|Default|SetInitial%20Speed (Variables|/Script/Engine.ProjectileMovementComponent|GetInitialSpeed _asprojectile_movement_component)))
                  (CallFunction|DebugMessage "Velocity" (Utilities|String|ToString(Float) _output_get))
                  (bind _output_get_2 (Variables|Default|SetOverride%20Gravity%20Z (* (Class|GameFunctionLibrary|GetGlobalGravityZ self) (Variables|/Script/Engine.ProjectileMovementComponent|GetProjectileGravityScale _asprojectile_movement_component))))
                  (CallFunction|DebugMessage "Gravity" (Utilities|String|ToString(Float) _output_get_2))
                  (if (Math|Float|NearlyEqual(Float) (Variables|Default|GetOverride%20Gravity%20Z) 0.0 1e-06)
                    (Variables|Default|SetHasProjectile false)
                    (else
                      (Variables|Default|SetHasProjectile true))))
                (:CastFailed
                  (Variables|Default|SetHasProjectile false :!label _label))))
            (:CastFailed
              (goto _label))))
        (:Is%20Not%20Valid
          (goto _label))))
    (:CastFailed
      (goto _label))))

(event Custom|CustomEvent_2
  (params (CurrentCount :type Integer))
  (Default|SetGrenadeCount (Variables|Default|GetAs%20MENU%20HUDTesting) CurrentCount))

(event Custom|CustomEvent_3
  (params (CurrentCount :type Integer) (Inventory :type Inventory%20Component%20Object%20Reference))
  (Default|SetFlareCount (Variables|Default|GetAs%20MENU%20HUDTesting) CurrentCount))

(event Custom|CustomEvent_4
  (params (Item :type Item%20Object%20Reference))
  (Default|RefleshWeaponHud (Variables|Default|GetAs%20MENU%20HUDTesting) Item)
  (CallFunction|HasValidProjectile Item))

(event Custom|CustomEvent
  (params (ClipCount :type Integer))
  (Default|SetClipCountR(SWS) (Variables|Default|GetAs%20MENU%20HUDTesting) (Utilities|Text|ToText(Integer) ClipCount)))

(event Custom|OnClipCountChanged_Event_0
  (params (ClipCount :type Integer))
  (Default|SetClipCountL(SWS) (Variables|Default|GetAs%20MENU%20HUDTesting) (Utilities|Text|ToText(Integer) ClipCount)))

(event Custom|CustomEvent_7
  (params (AmmoCount :type Integer))
  (Default|SetAmmoCountR(SWS) (Variables|Default|GetAs%20MENU%20HUDTesting) AmmoCount))

(event Custom|OnAmmoCountChanged_Event_0
  (params (AmmoCount :type Integer))
  (Default|SetAmmoCountL(SWS) (Variables|Default|GetAs%20MENU%20HUDTesting) AmmoCount))

(event Custom|OnAbillityChargeProgress_Event_1
  (params (aProgress :type Float%20%28single-precision%29) (aNextIndex :type Integer))
  (CallFunction|SetBoscoRocketCount aNextIndex))

(event Custom|OnReviveused_Event_0
  (params (ReviveCount :type Integer))
  (Default|SetBodyText (Variables|/Game/_DRGModding/Mod_3DHUD/MENU_HUDTesting.MENU_HUDTesting_C|GetCUI_BoscoInfos_Revive (Variables|Default|GetAs%20MENU%20HUDTesting)) (Utilities|Text|ToText(Integer) ReviveCount)))

(event Custom|OnAbillityChargeUsed_Event_0
  (params (aCurrentCharges :type Integer))
  (CallFunction|SetBoscoRocketCount aCurrentCharges))

(event Custom|OnAmmoChanged_Event_0
  (params (AmmoCount :type Integer))
  (Default|SetBodyText (Variables|/Game/_DRGModding/Mod_3DHUD/MENU_HUDTesting.MENU_HUDTesting_C|GetCUI_BoscoInfos_FAKIT (Variables|Default|GetAs%20MENU%20HUDTesting)) (Utilities|Text|ToText(Integer) AmmoCount)))

(event Custom|OnValueChanged%28Slider02%29
  (params (Vector :type Vector))
  (Transformation|SetActorRelativeRotation (Math|Conversions|RotationFromXVector Vector)))

(event Custom|OnValueChanged%28Slider01%29
  (params (Vector :type Vector))
  (Transformation|SetActorRelativeLocation Vector))

(event Custom|OnNewMessage
  (params (Message :type FSD%20Chat%20Message%20Structure%20%28by%20ref%29))
  (bind _msg (Utilities|IgnoreMsgbySender Message (Variables|Default|GetPlayer%20Character))
    (:CanProceed
      (|Outputs _msg) ; enters at OnReceiveChat
    )))

(fn GetModInfo
  (return "3D HUD" "Lesnov" "1.0.0"))

(fn GetModPages
  (return (Utilities|Array|MakeArray (Variables|Default|GetHUBMENU))))