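; Projectile prediction marker actor for the 3D HUD mod, drawn as a material billboard with a dynamic material instance made at construction.
; BeginPlay caches the local player character, with a separate lookup for running in the editor.
; Each tick maps player distance to a clamped factor, growing with distance, that drives actor scale, sprite size and a material parameter.
; Tick also prints debug strings.
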(event EventBeginPlay
  (Utilities|IsinDRG
    (:In%20DRG
      (bind _playercharacter (Utilities|GetLocalPlayerCharacter(Macro) true)
        (:Exec
          (Variables|Default|SetNewVar_0 _playercharacter))))
    (:In%20Editor
      (bind _returnvalue (Actor|GetActorOfClass "/Script/FSD.PlayerCharacter"))
      (Variables|Default|SetNewVar_0 _returnvalue))))

(event Collision|EventActorBeginOverlap
  (params (OtherActor :type Actor%20Object%20Reference)))

(event EventTick
  (params (DeltaSeconds :type Float%20%28single-precision%29))
  (bind _returnvalue (Transformation|GetActorLocation))
  (bind _newvar_0 (Variables|Default|GetNewVar_0))
  (bind _returnvalue_2 (Transformation|GetActorLocation _newvar_0))
  (bind _returnvalue_3 (Math|Vector|Distance(Vector) _returnvalue_2 _returnvalue))
  (bind _returnvalue_4 (Math|Float|MapRangeClamped _returnvalue_3 6e+02 3e+03 0.35 1.0))
  (bind _returnvalue_5 (* _returnvalue_4 32.0))
  (Utilities|IsValid _newvar_0
    (:Is%20Valid
      (Development|PrintString (Utilities|String|ToString(Float) _returnvalue_3) true true "(R=0.000000,G=0.660000,B=1.000000,A=1.000000)" 0.0)
      (Transformation|SetActorScale3D (Math|Conversions|ToVector(Float) _returnvalue_4))
      (Rendering|Material|SetScalarParameterValue (Variables|Default|GetNewVar_1) "Param" _returnvalue_4 :!class /Script/Engine.MaterialInstanceDynamic)
      (Utilities|Struct|SetmembersinMaterialSpriteElement (Utilities|Array|Get(acopy) (Variables|/Script/Engine.MaterialBillboardComponent|GetElements (Variables|Default|GetMaterialBillboard))) _returnvalue_5 _returnvalue_5))
    (:Is%20Not%20Valid
      (Development|PrintString "Hello"))))

(fn ConstructionScript
  (bind _returnvalue (Rendering|Material|CreateDynamicMaterialInstance "/Game/_DRGModding/Mod_3DHUD/MB_PredictProjectile_Inst.MB_PredictProjectile_Inst" "None" "None" :!class /Script/Engine.KismetMaterialLibrary))
  (bind _output_get (Variables|Default|SetNewVar_1 _returnvalue))
  (Utilities|Struct|SetmembersinMaterialSpriteElement (Utilities|Array|Get(acopy) (Variables|/Script/Engine.MaterialBillboardComponent|GetElements (Variables|Default|GetMaterialBillboard))) _output_get))