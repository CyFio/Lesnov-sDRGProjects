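; LEV Coin cosmetic prop for Deep Rock Galactic that changes facial expression by swapping eye meshes.
; Its parts are tinted through dynamic instances of a Bosco material.
; Using it shows a smile, then reverts to normal on a timer.
; Damage and hits feed a wait timer tied to the dead face, which fires a death call and later turns angry.
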(event OnComponentHit(LEVCoin_No_Eye)
  (params (HitComponent :type Primitive%20Component%20Object%20Reference) (OtherActor :type Actor%20Object%20Reference) (OtherComp :type Primitive%20Component%20Object%20Reference) (NormalImpulse :type Vector :default "0, 0, 0") (Hit :type Hit%20Result%20Structure%20%28by%20ref%29))
  (Utilities|WaitExec(Timer) 5.0 (delegate Custom|CustomEvent_1))
  (CallFunction|SetLEVState "NewEnumerator2")
  (CallFunction|SetLEVStatebyTimer "NewEnumerator3")
  (Development|PrintString "lev"))

(event OnUsedby(InstantUsable)
  (params (User :type Player%20Character%20Object%20Reference) (Key :type EInputKeys%20Enum :default "Use"))
  (CallFunction|SetLEVState "NewEnumerator1")
  (CallFunction|SetLEVStatebyTimer "NewEnumerator0"))

(event OnDamageTaken(SimpleHealth)
  (params (Amount :type Float%20%28single-precision%29))
  (Utilities|WaitExec(Timer) 5.0 (delegate Custom|CustomEvent_1))
  (CallFunction|SetLEVState "NewEnumerator2")
  (CallFunction|SetLEVStatebyTimer "NewEnumerator3")
  (Development|PrintString "lev"))

(event Custom|SetLEVStateByTimer
  (params (LEVState :type E_LEVState%20Enum :default "NewEnumerator0"))
  (Variables|Default|SetLastLEVState LEVState)
  (Utilities|Time|SetTimerbyEvent (delegate Custom|CustomEvent_0) 3.0))

(event Custom|CustomEvent_0
  (CallFunction|SetLEVState (Variables|Default|GetLastLEVState)))

(event Custom|CustomEvent_1
  (Utilities|WaitExec(Timer) 5.0 (delegate Custom|CustomEvent_1)) ; enters at OnExecFinished
)

(event EventBeginPlay
  (CallFunction|NewFunction0 "(R=1.000000,G=1.000000,B=1.000000,A=1.000000)" (Variables|Default|GetLEVCoin_WhileLine))
  (for _array_element (Utilities|Array|MakeArray (Variables|Default|GetLEVCoin_EYE) (Variables|Default|GetLEVCoin_BlackLine))
    (CallFunction|NewFunction0 :Target _array_element))
  (CallFunction|NewFunction0 "(R=0.000000,G=1.000000,B=0.193226,A=1.000000)" (Variables|Default|GetLEVCoin_No_Eye)))

(fn ConstructionScript
  (bind _returnvalue (Rendering|Material|CreateDynamicMaterialInstance "/Game/GameElements/Drone/Skins/SkinAssets/M_Bosco_PJ_Default.M_Bosco_PJ_Default" "None" "None" :!class /Script/Engine.KismetMaterialLibrary))
  (Rendering|Material|SetMaterial (Variables|Default|GetLEVCoin_No_Eye) 0 _returnvalue)
  (Rendering|Material|SetVectorParameterValue _returnvalue "DIFF || TintPrimary - Armor1" (Variables|Default|GetValue) :!class /Script/Engine.MaterialInstanceDynamic))

(fn SetLEVState
  (params (LEVState :type E_LEVState%20Enum :default "NewEnumerator0"))
  (bind _levcoin_eye (Variables|Default|GetLEVCoin_EYE))
  (switch Utilities|FlowControl|Switch|SwitchonE_LEVState LEVState
    (:NewEnumerator0
      (Components|StaticMesh|SetStaticMesh _levcoin_eye "/Game/_DRGModding/_Cosmetics/LEVCoin/LEVCoin_EYE_NORMAL.LEVCoin_EYE_NORMAL"))
    (:NewEnumerator1
      (Components|StaticMesh|SetStaticMesh _levcoin_eye "/Game/_DRGModding/_Cosmetics/LEVCoin/LEVCoin_EYE_SMILE.LEVCoin_EYE_SMILE"))
    (:NewEnumerator2
      (Components|StaticMesh|SetStaticMesh _levcoin_eye "/Game/_DRGModding/_Cosmetics/LEVCoin/LEVCoin_EYE_DIED.LEVCoin_EYE_DIED")
      (Default|CallOnLEVDead))
    (:NewEnumerator3
      (Components|StaticMesh|SetStaticMesh _levcoin_eye "/Game/_DRGModding/_Cosmetics/LEVCoin/LEVCoin_EYE_ANGRY.LEVCoin_EYE_ANGRY"))))

(fn NewFunction0
  (params (InputPin :type Linear%20Color%20Structure) (Target :type Primitive%20Component%20Object%20Reference))
  (bind _returnvalue (Rendering|Material|CreateDynamicMaterialInstance "/Game/GameElements/Drone/Skins/SkinAssets/M_Bosco_PJ_Default.M_Bosco_PJ_Default" "None" "None" :!class /Script/Engine.KismetMaterialLibrary))
  (Rendering|Material|SetMaterial Target 0 _returnvalue)
  (Rendering|Material|SetVectorParameterValue _returnvalue "DIFF || TintPrimary - Armor1" InputPin :!class /Script/Engine.MaterialInstanceDynamic)
  (Rendering|Material|SetVectorParameterValue _returnvalue "DIFF || TintPrimary - Armor2" InputPin :!class /Script/Engine.MaterialInstanceDynamic))