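; Deep Rock Galactic "Focus ADS" mod actor that adds aim-down-sights animation to the M1000 while charging a focus shot.
; Holding Fire starts a timed ADS montage that optionally fades the crosshair; release, sprint, item switch, reload or focus loss cancels it.
; Full focus swaps the fire montage and lights emissive parameters through a dynamic material.
; Input is active only with the M1000 equipped, and a hub menu edits saved settings.
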(event Custom|Save
  (Utilities|SavetoSlot(Macro) (Variables|Default|GetAs%20FADSavegame))
  (if (Variables|/Game/_DRGModding/Mod_FocusADS/FADSavegame.FADSavegame_C|GetDisableAutoHide (Variables|Default|GetAs%20FADSavegame))
    (Utilities|IsValid (Variables|FocusADS-Variables|GetAs%20WPN%20M1000)
      (:Is%20Valid
        (CallFunction|EnableCrosshair)))))

(event Custom|EnableCrosshair
  (bind _crosshair (Variables|Default|GetCrosshair))
  (bind _colorandopacity (Variables|/Script/UMG.UserWidget|GetColorAndOpacity _crosshair))
  ;[1 1 1] Toggle Crosshair Visibillity
  (if (not (Variables|/Game/_DRGModding/Mod_FocusADS/FADSavegame.FADSavegame_C|GetDisableAutoHide (Variables|Default|GetAs%20FADSavegame)))
    (Components|Timeline|SetPlayRate (Variables|Default|GetTL_Crosshair) 0.5)
    (bind _newtrack_0 (Timeline|TL_Crosshair Reverse)
      (:Update
        (Appearance|SetColorandOpacity _crosshair (Utilities|Struct|MakeLinearColor (.r _colorandopacity) (.g _colorandopacity) (.b _colorandopacity) (Math|Float|Lerp 1.0 0.0 _newtrack_0)) :!class /Script/UMG.UserWidget)))))

(event Custom|OnCheckClipCount
  (params (Amount :type Integer))
  ;[1 1 1] On Check Clip Count - Check if reloading is completed or not.
  (if (> Amount (Variables|FocusADS-Variables|GetClip%20Count))
    (Variables|FocusADS-Variables|SetIsReloading false)))

(event Custom|OnFinished%28ADS%29
  ;[1 1 1] OnFinished(ADS) - Disable ADS
  (Animation|Montage|MontageStop (Components|SkeletalMesh|GetAnimInstance (Variables|/Script/FSD.PlayerCharacter|GetFPMesh (Variables|FocusADS-Variables|GetPlayer%20Character))) 0.2 (Variables|FocusADS-Settings|GetMontage%28ADS%29))
  (Utilities|Time|ClearandInvalidateTimerbyHandle (Variables|FocusADS-Variables|GetTimer%28ADS%29)))

(event Custom|DisableCrosshair
  (bind _crosshair (Variables|Default|GetCrosshair))
  (bind _colorandopacity (Variables|/Script/UMG.UserWidget|GetColorAndOpacity _crosshair))
  ;[1 1 1] Toggle Crosshair Visibillity
  (if (not (Variables|/Game/_DRGModding/Mod_FocusADS/FADSavegame.FADSavegame_C|GetDisableAutoHide (Variables|Default|GetAs%20FADSavegame)))
    (Components|Timeline|SetPlayRate (Variables|Default|GetTL_Crosshair) 1.0)
    (bind _newtrack_0 (Timeline|TL_Crosshair Play)
      (:Update
        (Appearance|SetColorandOpacity _crosshair (Utilities|Struct|MakeLinearColor (.r _colorandopacity) (.g _colorandopacity) (.b _colorandopacity) (Math|Float|Lerp 1.0 0.0 _newtrack_0)) :!class /Script/UMG.UserWidget)))))

(event Custom|OnFullyFocused
  ;[1 1 1] Focus Related Event
  (CallFunction|ActivateEmissive)
  (Variables|/Script/FSD.AmmoDrivenWeapon|SetFP_FireAnimation (Variables|FocusADS-Variables|GetAs%20WPN%20M1000) "/Game/_DRGModding/Mod_FocusADS/Animations/ADS_Fire_Montage.ADS_Fire_Montage")
  (CallFunction|ToggleFPWidgetOpacity true))

(event Custom|OnFocusLost
  ;[1 1 1] Focus Related Event
  (CallFunction|DeactivateEmissive)
  (CallFunction|OnFinished(ADS))
  (CallFunction|ReverttoNonADS)
  (Utilities|FlowControl|Delay 0.4)
  (Variables|/Script/FSD.AmmoDrivenWeapon|SetFP_FireAnimation (Variables|FocusADS-Variables|GetAs%20WPN%20M1000) (Variables|FocusADS-Settings|GetMontage%28ADS%20-%20Fire%29)))

(event Custom|OnShotFired
  ;[1 1 1] OnShotFired
  (CallFunction|ToggleFPWidgetOpacity true))

(event Custom|OnItemEquipped_Event_0
  (params (Item :type Item%20Object%20Reference))
  ;[1 1 1] On item equipped, toggle input based on the current item
  (CallFunction|ToggleInputbyItem Item)
  (CallFunction|ReverttoNonADS))

(event Custom|OnADS
  ;[1 1 1] Fire Input - Toggle ADS based on focus shot condition
  (CallFunction|DebugMessage "OnADS")
  (Animation|Montage|PlayMontage (Variables|/Script/FSD.PlayerCharacter|GetFPMesh (Variables|FocusADS-Variables|GetPlayer%20Character)) (Variables|FocusADS-Settings|GetMontage%28ADS%29)
    (:then
      (CallFunction|DisableCrosshair)
      (CallFunction|ToggleFPWidgetOpacity false))))

(event Custom|OnRealodingEvent
  ;[1 1 1] OnReloading Event - Get the clip count before reloading and then, prepare the bool var for the ADS condition.
  (CallFunction|DebugMessage "OnReloadingEvent")
  (Variables|FocusADS-Variables|SetClip%20Count (Variables|/Script/FSD.AmmoDrivenWeapon|GetClipCount (Variables|FocusADS-Variables|GetAs%20WPN%20M1000)))
  (Variables|FocusADS-Variables|SetIsReloading true)
  (CallFunction|OnFinished(ADS))
  (CallFunction|ReverttoNonADS))

(event EventBeginPlay
  (bind _as_wpn_m1000 (Variables|FocusADS-Variables|GetAs%20WPN%20M1000))
  (bind _as_wpn_m1000_2 (Variables|FocusADS-Variables|GetAs%20WPN%20M1000))
  ;[1 1 1] Begin Play
  (bind _returnvalue (UserInterface|CreateWidget "/Game/_DRGModding/Mod_FocusADS/HUBMENU_FocusADS.HUBMENU_FocusADS_C"))
  (Variables|Default|SetAs%20HUBMENU%20Focus%20ADS _returnvalue)
  (bind _outputpin (Utilities|HandleSaveGame "/Game/_DRGModding/Mod_FocusADS/FADSavegame.FADSavegame_C")
    (:then
      (bind _asfadsavegame (Utilities|Casting|CastToFADSavegame _outputpin))
      (bind _output_get (Variables|Default|SetAs%20FADSavegame _asfadsavegame))
      (Default|EventInitialize (Variables|Default|GetAs%20HUBMENU%20Focus%20ADS) _output_get)
      (EventDispatchers|BindEventtoOnSavegameChanged (Variables|Default|GetAs%20HUBMENU%20Focus%20ADS) (delegate Custom|Save))
      (Initialization|Initialize)
      ;[1 1 1] Binding
      (EventDispatchers|BindEventtoFullyFocusedEvent _as_wpn_m1000 (EventDispatchers|CreateEvent :!event Custom|OnFullyFocused))
      (EventDispatchers|BindEventtoFocusLostEvent _as_wpn_m1000 (EventDispatchers|CreateEvent :!event Custom|OnFocusLost))
      (EventDispatchers|AssignOnItemEquipped (Variables|/Script/FSD.PlayerCharacter|GetInventoryComponent (Variables|FocusADS-Variables|GetPlayer%20Character)) (EventDispatchers|CreateEvent :!event Custom|OnItemEquipped_Event_0))
      (EventDispatchers|BindEventtoOnReloadingEvent _as_wpn_m1000_2 (EventDispatchers|CreateEvent :!event Custom|OnRealodingEvent))
      (EventDispatchers|BindEventtoOnClipCountChanged _as_wpn_m1000_2 (EventDispatchers|CreateEvent :!event Custom|OnCheckClipCount))
      (EventDispatchers|BindEventtoOnShotFiredEvent _as_wpn_m1000_2 (EventDispatchers|CreateEvent :!event Custom|OnShotFired)))))

(event Input|ActionEvents|InputActionFire
  (params (Key :type Key%20Structure :default "None"))
  ;[1 1 1] Fire Input - Toggle ADS based on focus shot condition
  (:Pressed
    (if (not (Variables|FocusADS-Variables|GetIsReloading))
      (bind _returnvalue (Utilities|Time|SetTimerbyEvent (delegate Custom|OnADS) (Variables|FocusADS-Settings|GetADSStartTime)))
      (Variables|FocusADS-Variables|SetTimer%28ADS%29 _returnvalue)))
  (:Released
    (CallFunction|OnFinished(ADS))))

(event Input|ActionEvents|InputActionRun
  (params (Key :type Key%20Structure :default "None"))
  ;[1 1 1] Disable ADS by inputs.
  ; Maybe Focus Lost Event is enough.
  (:Pressed
    (CallFunction|OnFinished(ADS))
    (CallFunction|ReverttoNonADS)))

(event Input|ActionEvents|InputActionCycleitem
  (params (Key :type Key%20Structure :default "None"))
  ;[1 1 1] Disable ADS by inputs.
  ; Maybe Focus Lost Event is enough.
  (:Pressed
    (CallFunction|OnFinished(ADS))
    (CallFunction|ReverttoNonADS)))

(fn ConstructionScript)

(fn DebugMessage
  (params (Sender :type String) (Text :type String))
  (Utilities|PrintViaChat (Variables|FocusADS-Settings|GetDisable%20Debug) (Utilities|QuickAppend(Macro) "FADS" Sender) Text "NormalUser"))

(fn DeactivateEmissive
  (for _array_element (Variables|FocusADS-Variables|GetParameter%20Name)
    (Rendering|Material|SetScalarParameterValue (Variables|FocusADS-Variables|GetDMI) _array_element 0.0 :!class /Script/Engine.MaterialInstanceDynamic)))

(fn ActivateEmissive
  (CallFunction|DebugMessage "Activate Emissive")
  (for _array_element (Variables|FocusADS-Variables|GetParameter%20Name)
    (if (.ReturnValue (Utilities|Map|Find (Variables|FocusADS-Variables|GetDefaultParameterValues) _array_element))
      (Rendering|Material|SetScalarParameterValue (Variables|FocusADS-Variables|GetDMI) _array_element (.Value (Utilities|Map|Find (Variables|FocusADS-Variables|GetDefaultParameterValues) _array_element)) :!class /Script/Engine.MaterialInstanceDynamic))))

(fn ToggleInputbyItem
  (params (Item :type Object%20Object%20Reference))
  (if (== Item (Variables|FocusADS-Variables|GetAs%20WPN%20M1000))
    (Input|EnableInput (Variables|FocusADS-Variables|GetFSDPlayer%20Controller))
    (Variables|FocusADS-Variables|SetIsReloading false)
    (else
      (Input|DisableInput (Variables|FocusADS-Variables|GetFSDPlayer%20Controller)))))

(fn ToggleFPWidgetOpacity
  (params (Show :type Boolean))
  (bind _as_wpn_m1000 (Variables|FocusADS-Variables|GetAs%20WPN%20M1000))
  (bind _firstpersonwidget (Variables|/Game/WeaponsNTools/BoltActionRifle/WPN_M1000.WPN_M1000_C|GetFirstPersonWidget _as_wpn_m1000))
  (bind _returnvalue (UserInterface|GetWidget _firstpersonwidget))
  (bind _colorandopacity (Variables|/Script/UMG.UserWidget|GetColorAndOpacity _returnvalue))
  (Appearance|SetColorandOpacity _returnvalue (Utilities|Struct|MakeLinearColor (.r _colorandopacity) (.g _colorandopacity) (.b _colorandopacity) (Math|Float|SelectFloat 1.0 0.01 Show)) :!class /Script/UMG.UserWidget))

(fn ReverttoNonADS
  (CallFunction|EnableCrosshair)
  (CallFunction|ToggleFPWidgetOpacity true))

(event Custom|OnPlayerCharacterPossesed
  (CallFunction|DebugMessage "OnPossesed")
  (bind _playercharacter (Utilities|GetLocalPlayerCharacter(Macro) true)
    (:Exec
      (bind _output_get (Variables|FocusADS-Variables|SetPlayer%20Character _playercharacter))
      (Utilities|WaitUntilValid(Inventory-Items|EditorSkip) _output_get
        (:Found
          (bind _founditem (Utilities|FindItemfromClass _output_get "/Game/WeaponsNTools/BoltActionRifle/WPN_M1000.WPN_M1000_C")
            (:Found
              (bind _aswpn_m1000 (Utilities|Casting|CastToWPN_M1000 _founditem))
              (Variables|FocusADS-Variables|SetAs%20WPN%20M1000 _aswpn_m1000)
              (Variables|FocusADS-Settings|SetMontage%28ADS%20-%20Fire%29 (Variables|/Script/FSD.AmmoDrivenWeapon|GetFP_FireAnimation (Variables|FocusADS-Variables|GetAs%20WPN%20M1000)))
              (|DMIInitialize)
              (if (== (Utilities|GetCurrentItem (Variables|FocusADS-Variables|GetPlayer%20Character)) (Variables|FocusADS-Variables|GetAs%20WPN%20M1000))
                (Input|EnableInput (Variables|FocusADS-Variables|GetFSDPlayer%20Controller)))
              (Variables|Default|SetCrosshair (Class|CrosshairAggregator|GetorCreateCrosshair (Variables|/Game/WeaponsNTools/BoltActionRifle/WPN_M1000.WPN_M1000_C|GetCrosshairAggregator (Variables|FocusADS-Variables|GetAs%20WPN%20M1000))))
              (return))
            (:NotFound
              (CallFunction|DebugMessage "WPN_M1000" "is not equipped"))))))))

(fn GetModInfo
  (return "Focus ADS" "Lesnov" "1.1.1"))

(fn GetModPages
  (return (Utilities|Array|MakeArray (Variables|Default|GetAs%20HUBMENU%20Focus%20ADS))))