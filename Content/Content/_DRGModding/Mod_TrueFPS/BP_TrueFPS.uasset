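; Deep Rock Galactic mod actor that gives the local player a visible body and legs in first person.
; It attaches an extra skeletal mesh to the capsule, copying equipped armor, anim class and third-person montages, and hides it outside first-person view.
; Possession re-adds the mesh and closing the wardrobe refreshes it.
; "!TF" chat commands toggle saved body-bone hiding and debug messages, re-add the mesh or print info.
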(event Custom|AddMesh%28Legs%29
  ;[1 1 1] Add the leg mesh to player character and transfer some vanity stuff from equipped vanity.
  (Utilities|PreventExecutionWhileRunning :!label _label)
  (Utilities|Array|Add)
  (goto _label ExecFinish))

(event Custom|CustomEvent_1
  ;[1 1 1] When different player character is possessed, call add mesh again.
  (CallFunction|AddMesh(Legs)))

(event Custom|CustomEvent_3
  (params (Window :type Window%20Widget%20Object%20Reference))
  (Utilities|FlowControl|Delay 0.5)
  (CallFunction|TransferMeshfromPlayerCharacterVanity)
  (CallFunction|AttachLegMeshtoPlayerCharacter))

(event EventBeginPlay
  (|Create|LoadSaveGame)
  (|ValidChecking(Armorrelatedvanities)
    (:OutputPin
      ;[1 1 1] When different player character is possessed, call add mesh again.
      (bind _fsdplayercontroller (Utilities|GetLocalPlayerController(Macro) true)
        (:Completed
          (EventDispatchers|BindEventtoOnPlayerCharacterPossesed _fsdplayercontroller (delegate Custom|CustomEvent_1))
          (CallFunction|PrintDebugMsg "PlayerController" "Finished")
          (bind _foundwidgets (Widget|GetAllWidgetsOfClass "/Game/UI/Menu_Wardrobe/_MENU_Wardrobe._MENU_Wardrobe_C" false))
          (EventDispatchers|BindEventtoOnWindowClosed (Utilities|Array|Get(acopy) _foundwidgets) (delegate Custom|CustomEvent_3))
          (|QuickConsoleCommand(TFPS)) ; Used to implement console command quickly via chat
          (CallFunction|AddMesh(Legs)))))))

(fn ConstructionScript)

(fn TransferMeshfromPlayerCharacterVanity
  (Utilities|IsinDRG
    (:In%20DRG
      (|InDRG))
    (:In%20Editor
      (Editor|InEditor))))

(fn AttachLegMeshtoPlayerCharacter
  (bind _player_character (Variables|TrueFPS|GetPlayer%20Character))
  (bind _addedmeshcomp (Variables|Default|GetAddedMeshComp))
  (bind _capsulecomponent (Variables|/Script/Engine.Character|GetCapsuleComponent _player_character))
  (Utilities|IsValid _player_character
    (:Is%20Valid
      (Transformation|AttachComponentToComponent _addedmeshcomp _capsulecomponent "None" "SnapToTarget" "SnapToTarget" "SnapToTarget" true)
      (Transformation|SetRelativeLocation _addedmeshcomp (Math|Vector|MakeVector (Math|Float|SelectFloat 8e+01 (Variables|TrueFPS|GetForwardOffset) (Variables|TrueFPSDebug-Settings|GetEnableDebugPosition)) 0.0 (* (* (Components|Capsule|GetScaledCapsuleHalfHeight _capsulecomponent) (Variables|TrueFPS|GetHalfHeightScale)) -1.0)) false false)
      (Transformation|SetRelativeRotation _addedmeshcomp "0.000000,-90.000000,0.000000" false false)
      (if (Variables|/Game/_DRGModding/Mod_TrueFPS/TFPSSavegame.TFPSSavegame_C|GetDisableBodyMesh (Variables|TrueFPS|GetAs%20TFPSSavegame))
        (CallFunction|HideBodyMesh)))))

(fn PrepareLegMesh
  (bind _player_character (Variables|TrueFPS|GetPlayer%20Character))
  (bind _returnvalue (AddComponent|AddFirstPersonSkeletalMeshComponent _player_character false))
  (Variables|Default|SetAddedMeshComp _returnvalue)
  (CallFunction|TransferMeshfromPlayerCharacterVanity)
  (Class|SkeletalMeshComponent|SetAnimClass _returnvalue (Utilities|GetClass (Components|SkeletalMesh|GetAnimInstance (Variables|/Script/Engine.Character|GetMesh _player_character)))))

(fn BPTrueFPSAutoGenFunc
  (params (Montage :type Anim%20Montage%20Object%20Reference))
  (Animation|Montage|MontagePlay (Components|SkeletalMesh|GetAnimInstance (Variables|Default|GetAddedMeshComp)) Montage 1.0 "MontageLength" 0.0 true)
  (Utilities|PrintViaChat (Variables|TrueFPSDebug-Settings|GetDisableDebugMessage) "" (Utilities|GetDisplayName Montage) "NormalUser"))

(fn PrintQCCMsg
  (params (Text :type String))
  (Utilities|PrintViaChat false "TFPS" Text "Developer"))

(fn Save
  (Utilities|SavetoSlot(Macro) (Variables|TrueFPS|GetAs%20TFPSSavegame)))

(fn HideBodyMesh
  (for _array_element (Variables|TrueFPS|GetBoneNamesToHide)
    (Components|SkinnedMesh|HideBonebyName (Variables|Default|GetAddedMeshComp) _array_element "PBO_None")))

(fn UnhideBodyMesh
  (for _array_element (Variables|TrueFPS|GetBoneNamesToHide)
    (Components|SkinnedMesh|UnHideBonebyName (Variables|Default|GetAddedMeshComp) _array_element)))

(fn PrintDebugMsg
  (params (Sender :type String) (Text :type String))
  (Utilities|PrintViaChat (Variables|/Game/_DRGModding/Mod_TrueFPS/TFPSSavegame.TFPSSavegame_C|GetDisableDBMsg (Variables|TrueFPS|GetAs%20TFPSSavegame)) Sender Text "NormalUser"))

(event Custom|CustomEvent_0
  (params (NewCameraMode :type ECharacterCameraMode%20Enum :default "FirstPerson") (OldCameraMode :type ECharacterCameraMode%20Enum :default "FirstPerson"))
  (bind _addedmeshcomp (Variables|Default|GetAddedMeshComp))
  ;[1 1 1] The leg mesh's visibillity is changed based on camera view, so I can't see the mesh when TP view.
  (switch Utilities|FlowControl|Switch|SwitchonECharacterCameraMode NewCameraMode
    (:FirstPerson
      (Development|SetHiddeninGame _addedmeshcomp false false))
    (:ThirdPerson
      (Development|SetHiddeninGame _addedmeshcomp true false :!label _label))
    (:Follow
      (goto _label))
    (:DownCamera
      (goto _label))
    (:PhotographyMode
      (goto _label))))

(event Custom|CustomEvent_2
  ;[1 1 1] Obsolute, but it might be used when MENU_WARDEROBE stop working
  (Utilities|FlowControl|Delay 1.0)
  (CallFunction|TransferMeshfromPlayerCharacterVanity)
  (CallFunction|AttachLegMeshtoPlayerCharacter))

(event Custom|OnNewMessage
  (params (Message :type FSD%20Chat%20Message%20Structure%20%28by%20ref%29))
  (bind _msg (Utilities|IgnoreMsgbySender Message (Variables|TrueFPS|GetPlayer%20Character))
    (:CanProceed
      (|Outputs _msg) ; enters at OnReceiveChat
    )))