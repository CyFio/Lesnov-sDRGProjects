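; Deep Rock Galactic mod actor that gives the local player a pair of shoulder weapons on the first-person camera.
; It spawns the saved weapon class as mirrored actors, refilled on resupply and hidden outside first person.
; One input equips or alternately fires on tap; holding holsters, or toggles the selection menu in the Space Rig.
; The menu is built from data assets found by path, and a chat command opens a transform-tuning helper.
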(event Custom|OnInitialize
  (params (IsInSpacerig :type Boolean))
  (Variables|Default|SetIs%20in%20Spacerig IsInSpacerig)
  (if (Variables|Settings-Debug|GetForceInCave)
    (Development|PrintString "Force In Cave is active" true true "(R=0.000000,G=0.660000,B=1.000000,A=1.000000)" 5.0)
    (Variables|Default|SetIs%20in%20Spacerig false))
  (Debug|DebugMessage "SW Spawned")
  (|InitializeVariables)
  (|HandleSavegame)
  (|CreateWeaponSelecterMenu)
  (|LoadSWPNs
    (:Completed
      (Utilities|IsinDRG
        (:In%20DRG
          (CallFunction|InitializeWeapon (Variables|/Game/_DRGModding/Mod_ShoulderWeaponSystem/ShoulderWeaponData_Base.ShoulderWeaponData_Base_C|GetWeaponClass (Variables|/Game/_DRGModding/Mod_ShoulderWeaponSystem/SWSavegame.SWSavegame_C|GetSelectedWeapon (Variables|Default|GetAs%20SWSavegame))))
          (Variables|Default|SetInitializeFinished true)
          (Debug|DebugMessage "Initialization " "Finished")
          (|QuickConsoleCommand(TFPS)_2_2) ; Used to implement console command quickly via chat
        )
        (:In%20Editor
          (Debug|SpawnWeaponbyClass (Variables|Settings-Debug|GetDebugSpawnWeapon))
          (Input|EnableInput (Game|GetPlayerController 0)))))))

(event Custom|CustomEvent_0
  ;[1 1 1] Input - Shoulder Weapon (Handle Toggle equipping, Fire, Show HUD)
  (Variables|Default|SetEquippedByTimer true)
  (CallFunction|DeactivateShoulderWeapon))

(event Custom|ToggleShoulderWeapon
  ;[1 1 1] Toggle Shoulder Weapon Anim
  (if (Variables|Default|GetIsEquipped)
    (Variables|Default|SetIsEquipped false)
    (CallFunction|ToggleWeaponInput false)
    (bind _newtrack_0 (Timeline|Timeline_0 Reverse)
      (:Update
        (Transformation|SetRelativeRotation (Variables|Default|GetAP_Weapon) (Math|Rotator|MakeRotator 0.0 (Math|Float|Lerp 9e+01 0.0 _newtrack_0) 0.0) false false)))
    (else
      (Variables|Default|SetIsEquipped true)
      (CallFunction|ToggleWeaponInput true)
      (Timeline|Timeline_0 Play))))

(event Custom|ChangeWeapon
  ;[1 1 1] Event - Change Weapon
  (CallFunction|InitializeWeapon (Variables|/Game/_DRGModding/Mod_ShoulderWeaponSystem/ShoulderWeaponData_Base.ShoulderWeaponData_Base_C|GetWeaponClass (Variables|/Game/_DRGModding/Mod_ShoulderWeaponSystem/SWSavegame.SWSavegame_C|GetSelectedWeapon (Variables|Default|GetAs%20SWSavegame)))))

(event Custom|OnTryWeaponFire
  (if (Variables|Default|GetIsEquipped)
    (if (Variables|Default|GetIsRightFired)
      (if (> (Variables|/Game/_DRGModding/Mod_ShoulderWeaponSystem/BP_ShoulderWeaponBase.BP_ShoulderWeaponBase_C|GetClipSize%28Current%29 (Variables|Default|GetAttached%20Weapon_L)) 0)
        (CallFunction|FireWeapon (Variables|Default|GetAttached%20Weapon_L))
        (Variables|Default|SetIsRightFired false)
        (else
          (CallFunction|FireWeapon (Variables|Default|GetAttachedWeapon_R))
          (Variables|Default|SetIsRightFired true)))
      (elif (> (Variables|/Game/_DRGModding/Mod_ShoulderWeaponSystem/BP_ShoulderWeaponBase.BP_ShoulderWeaponBase_C|GetClipSize%28Current%29 (Variables|Default|GetAttachedWeapon_R)) 0)
        (CallFunction|FireWeapon (Variables|Default|GetAttachedWeapon_R))
        (Variables|Default|SetIsRightFired true)
        (else
          (CallFunction|FireWeapon (Variables|Default|GetAttached%20Weapon_L))
          (Variables|Default|SetIsRightFired false))))))

(event Custom|DeactivateShoulderWeapon
  ;[1 1 1] Toggle Shoulder Weapon Anim
  (Variables|Default|SetIsEquipped false)
  (CallFunction|ToggleWeaponInput false)
  (bind _newtrack_0 (Timeline|Timeline_0 Reverse)
    (:Update
      (Transformation|SetRelativeRotation (Variables|Default|GetAP_Weapon) (Math|Rotator|MakeRotator 0.0 (Math|Float|Lerp 9e+01 0.0 _newtrack_0) 0.0) false false))))

(event Custom|PlayBaseFireAnimation
  ;[1 1 1] Base Fire Anim
  (Components|Timeline|SetPlayRate (Variables|Default|GetTL_BaseFireAnim) (Variables|Default|GetPlayRateByFireRate))
  (bind _newtrack_0 (Timeline|TL_BaseFireAnim PlayFromStart)
    (:Update
      (Transformation|SetActorRelativeLocation (Math|Vector|Lerp(Vector) "0, 0, 0" "12.000000, 0, 0" _newtrack_0)))))

(event Custom|ActivateShoulderweapon
  ;[1 1 1] Toggle Shoulder Weapon Anim
  (Variables|Default|SetIsEquipped true)
  (CallFunction|ToggleWeaponInput true)
  (bind _newtrack_0 (Timeline|Timeline_0 Play)
    (:Update
      (Transformation|SetRelativeRotation (Variables|Default|GetAP_Weapon) (Math|Rotator|MakeRotator 0.0 (Math|Float|Lerp 9e+01 0.0 _newtrack_0) 0.0) false false))))

(event Input|ActionEvents|InputActionShoulderWeapon
  (params (Key :type Key%20Structure :default "None"))
  ;[1 1 1] Input - Shoulder Weapon (Handle Toggle equipping, Fire, Show HUD)
  (:Pressed
    (|Show(hud-spacerig)
      (:false
        (bind _returnvalue (Utilities|Time|SetTimerbyEvent (delegate Custom|CustomEvent_0) 0.5))
        (Variables|Default|SetTimerSelection _returnvalue))))
  (:Released
    (if (Variables|Default|GetEquippedByTimer)
      (Variables|Default|SetEquippedByTimer false)
      (if (Variables|Default|GetIsMenuOpened)
        (if (Variables|Default|GetIsMenuOpened) :!label _label
          (Variables|Default|SetIsMenuOpened false :!label _label_2)
          (else
            (if (Variables|Default|GetIsEquipped) :!label _label_3
              (CallFunction|OnTryWeaponFire)
              (else
                (CallFunction|ActivateShoulderweapon)
                (goto _label_2))))))
      (elif (Utilities|Time|IsValidTimerHandle (Variables|Default|GetTimerSelection))
        (Utilities|Time|ClearandInvalidateTimerbyHandle (Variables|Default|GetTimerSelection))
        (goto _label)
        (else
          (goto _label_3))))))

(fn ConstructionScript)

(fn InitializeWeapon
  (params (Class :type BP%20Shoulder%20Weapon%20Base%20Class%20Reference))
  (bind _attached_weapon_l (Variables|Default|GetAttached%20Weapon_L))
  (bind _attachedweapon_r (Variables|Default|GetAttachedWeapon_R))
  (Utilities|IsValid _attachedweapon_r
    (:Is%20Valid
      (Actor|DestroyActor _attachedweapon_r))
    (:Is%20Not%20Valid
      _))
  (Utilities|IsValid _attached_weapon_l
    (:Is%20Valid
      (Actor|DestroyActor _attached_weapon_l))
    (:Is%20Not%20Valid
      _))
  (bind _attachedweapon_r_2 (CallFunction|SpawnWeapon Class (Variables|Default|GetAttachedWeapon_R) true))
  (CallFunction|TransferMaterialfromPrimaryWeapon _attachedweapon_r_2)
  (Variables|Default|SetPlayRateByFireRate (Math|Float|SafeDivide 1.0 (Variables|/Game/_DRGModding/Mod_ShoulderWeaponSystem/BP_ShoulderWeaponBase.BP_ShoulderWeaponBase_C|GetFireCooldown (Variables|Default|GetAttachedWeapon_R))))
  (bind _attachedweapon_r_3 (CallFunction|SpawnWeapon Class (Variables|Default|GetAttached%20Weapon_L) false))
  (CallFunction|TransferMaterialfromPrimaryWeapon _attachedweapon_r_3))

(fn ToggleWeaponInput
  (params (EnableInput :type Boolean))
  (bind _attachedweapon_r (Variables|Default|GetAttachedWeapon_R))
  (bind _fsdplayer_controller (Variables|Default|GetFSDPlayer%20Controller))
  (if EnableInput
    (Input|EnableInput _attachedweapon_r _fsdplayer_controller)
    (else
      (Input|DisableInput _attachedweapon_r _fsdplayer_controller))))

(fn SpawnWeaponbyClass
  (params (SWBase :type BP%20Shoulder%20Weapon%20Base%20Class%20Reference))
  (CallFunction|InitializeWeapon SWBase))

(fn DebugMessage
  (params (Sender :type String) (Text :type String))
  (Utilities|PrintViaChat false (Utilities|QuickAppend(Macro) "SWPN" Sender) Text "NormalUser"))

(fn ToggleMouseCursor
  (params (Condition :type Boolean))
  (bind _returnvalue (Game|GetPlayerController 0))
  (bind _fsdplayer_controller (Variables|Default|GetFSDPlayer%20Controller))
  (Utilities|IsinDRG
    (:In%20DRG
      (if Condition
        (Variables|/Script/Engine.PlayerController|SetbShowMouseCursor _fsdplayer_controller false)
        (else
          (Variables|/Script/Engine.PlayerController|SetbShowMouseCursor _fsdplayer_controller true))))
    (:In%20Editor
      (if Condition
        (Variables|/Script/Engine.PlayerController|SetbShowMouseCursor _returnvalue false)
        (else
          (Variables|/Script/Engine.PlayerController|SetbShowMouseCursor _returnvalue true))))))

(fn GetModInfo
  (return "" "" ""))

(fn GetModPages
  (return (Utilities|Array|MakeArray (Variables|Default|GetMODHUB_Widget))))

(fn TransferMaterialfromPrimaryWeapon
  (params (Target :type BP%20Shoulder%20Weapon%20Base%20Object%20Reference))
  (bind _primarymaterial (Variables|Default|GetPrimaryMaterial))
  (Utilities|IsValid _primarymaterial
    (:Is%20Valid
      (Rendering|Material|SetMaterial (Variables|/Game/_DRGModding/Mod_ShoulderWeaponSystem/BP_ShoulderWeaponBase.BP_ShoulderWeaponBase_C|GetShoulderWeapon Target) 0 _primarymaterial))))

(fn SpawnWeapon
  (params (Class :type BP%20Shoulder%20Weapon%20Base%20Class%20Reference) (AttachedWeapon :type BP%20Shoulder%20Weapon%20Base%20Object%20Reference%20%28by%20ref%29) (IsRightSide :type Boolean))
  (bind _firstpersonwidget (Variables|/Game/_DRGModding/Mod_ShoulderWeaponSystem/BP_ShoulderWeaponBase.BP_ShoulderWeaponBase_C|GetFirstPersonWidget AttachedWeapon))
  (bind _positionoffset (Variables|/Game/_DRGModding/Mod_ShoulderWeaponSystem/BP_ShoulderWeaponBase.BP_ShoulderWeaponBase_C|GetPositionOffset AttachedWeapon))
  (bind (_x _y _z) (Math|Vector|BreakVector _positionoffset))
  (bind _returnvalue (Game|SpawnActorfromClass Class (Math|Transform|MakeTransform "0, 0, 0" "0, 0, 0" "1,1,1") "AlwaysSpawn" 0 0))
  (|SetBy-RefVar AttachedWeapon _returnvalue)
  (Transformation|AttachComponentToComponent AttachedWeapon (Variables|Default|GetAP_Weapon) "None" "SnapToTarget" "KeepRelative" "KeepRelative" true)
  (Variables|/Game/_DRGModding/Mod_ShoulderWeaponSystem/BP_ShoulderWeaponBase.BP_ShoulderWeaponBase_C|SetShoulderWeaponSystem AttachedWeapon self)
  (Transformation|SetActorRelativeLocation AttachedWeapon (Math|Vector|SelectVector _positionoffset (Math|Vector|MakeVector _x (* -1 _y) _z) IsRightSide))
  (if IsRightSide
    _
    (else
      (Transformation|SetActorRelativeScale3D AttachedWeapon "1.000000,-1.000000,1.000000")
      (Transformation|SetRelativeScale3D _firstpersonwidget "0.030000,-0.030000,0.030000")
      (Class|WidgetComponent|SetPivot _firstpersonwidget (Math|Vector2D|MakeVector2D 1.0 0.0))))
  (return AttachedWeapon))

(fn FireWeapon
  (params (InputPin :type BP%20Shoulder%20Weapon%20Base%20Object%20Reference))
  (Utilities|IsValid InputPin
    (:Is%20Valid
      (if (Default|CanFire InputPin)
        (Default|OnWeaponFired InputPin)
        (CallFunction|PlayBaseFireAnimation)
        (Default|SpawnMuzzleEffect InputPin)
        (Default|PlaySound(Muzzle) InputPin false)
        (CallFunction|SpawnProjectile InputPin)
        (else
          (Default|PlaySound(Muzzle) InputPin true))))))

(fn SpawnProjectile
  (params (Target :type BP%20Shoulder%20Weapon%20Base%20Object%20Reference))
  (bind (_return_value_location _return_value_rotation) (Default|GetMuzzlePos Target))
  (Game|SpawnActorfromClass (Variables|/Game/_DRGModding/Mod_ShoulderWeaponSystem/BP_ShoulderWeaponBase.BP_ShoulderWeaponBase_C|GetProjectile Target) (Math|Transform|MakeTransform (+ _return_value_location (* (Math|Vector|GetForwardVector _return_value_rotation) (Variables|Settings-Projectile|GetSpawnOffset))) _return_value_rotation "1,1,1") "AlwaysSpawn" 0 0))

(event Custom|OnClicked_Event_0
  (params (ShoulderWeaponData :type Shoulder%20Weapon%20Data%20Base%20Object%20Reference) (CUI_Icon :type CUI%20Icon%20Object%20Reference))
  (Utilities|Initialized
    (:true
      (bind _alreadyselected (Default|IsAlreadySelected (Variables|Default|GetAs%20SWSavegame) ShoulderWeaponData))
      (if (not _alreadyselected)
        (Default|SetSelectedText (Variables|Default|GetAs%20CMENU%20SWSelection) (Variables|/Game/_DRGModding/Mod_ShoulderWeaponSystem/ShoulderWeaponData_Base.ShoulderWeaponData_Base_C|GetSelectedString ShoulderWeaponData))
        (Default|SetColor CUI_Icon true)
        (for _array_element (Variables|Default|GetShoulderWeaponList)
          (if (!= _array_element CUI_Icon)
            (Default|SetColor _array_element false)))
        (Utilities|SavetoSlot(Macro) (Variables|Default|GetAs%20SWSavegame))
        (CallFunction|ChangeWeapon)))))

(event Custom|OnResuppliedEvent_Event_0
  (params (percentage :type Float%20%28single-precision%29))
  (bind _attachedweapon_r (Variables|Default|GetAttachedWeapon_R))
  (bind _attached_weapon_l (Variables|Default|GetAttached%20Weapon_L))
  (Utilities|IsValid _attached_weapon_l
    (:Is%20Valid
      (Default|Refill _attached_weapon_l percentage))
    (:Is%20Not%20Valid
      _))
  (Utilities|IsValid _attachedweapon_r
    (:Is%20Valid
      (Default|Refill _attachedweapon_r percentage))))

(event Custom|OnCameraModeChanged_Event_0
  (params (NewCameraMode :type ECharacterCameraMode%20Enum :default "FirstPerson") (OldCameraMode :type ECharacterCameraMode%20Enum :default "FirstPerson"))
  (Utilities|FlowControl|Sequence
    (:then_0
      (if (Utilities|Enum|NotEqual(Enum) NewCameraMode "FirstPerson")
        (switch Utilities|FlowControl|Switch|SwitchonECharacterCameraMode NewCameraMode
          (:ThirdPerson
            _)
          (:Follow
            _)
          (:DownCamera
            _)
          (:PhotographyMode
            _))
        (bind (_attached_weapon_l _attachedweapon_r) (Utilities|Both)
          (:Is%20Valid
            (Rendering|SetActorHiddenInGame _attached_weapon_l true))
          (:Is%20Valid2
            (Rendering|SetActorHiddenInGame _attachedweapon_r true)))
        (else
          (bind (_attached_weapon_l_2 _attachedweapon_r_2) (Utilities|Both :!label _label)
            (:Is%20Valid
              (Rendering|SetActorHiddenInGame _attached_weapon_l_2 false))
            (:Is%20Valid2
              (Rendering|SetActorHiddenInGame _attachedweapon_r_2 false))))))
    (:then_1
      (Utilities|FlowControl|Delay 0.5)
      (if (Utilities|Enum|Equal(Enum) NewCameraMode "FirstPerson")
        (goto _label)))))

(event Custom|OnPlayerCharacterPossesed_Event_0
  (bind _playercharacter (Utilities|GetLocalPlayerCharacter(Macro) true)
    (:Exec
      (bind _output_get (Variables|Default|SetPlayer%20Character _playercharacter))
      (Transformation|AttachComponentToComponent (Variables|/Script/FSD.PlayerCharacter|GetFirstPersonCamera _output_get) "None" "SnapToTarget" "SnapToTarget" "KeepRelative" false))))

(event Custom|CustomEvent_1
  (Utilities|FlowControl|Delay 0.1)
  (bind (_attached_weapon_l _attachedweapon_r) (Utilities|Both)
    (:Is%20Valid
      (Rendering|SetActorHiddenInGame _attached_weapon_l false))
    (:Is%20Valid2
      (Rendering|SetActorHiddenInGame _attachedweapon_r false))))

(event Custom|ToggleSelectionMenu
  (bind _as_cmenu_swselection (Variables|Default|GetAs%20CMENU%20SWSelection))
  (bind _returnvalue (Widget|IsVisible _as_cmenu_swselection))
  (bind _returnvalue_2 (select _returnvalue "Collapsed" "SelfHitTestInvisible"))
  (Variables|Default|SetIsMenuOpened true)
  (if _returnvalue
    (CallFunction|DeactivateShoulderWeapon)
    (else
      (CallFunction|ActivateShoulderweapon)))
  (CallFunction|ToggleMouseCursor _returnvalue)
  (Widget|SetVisibility (Variables|Default|GetAs%20CMENU%20SWSelection) _returnvalue_2)
  (switch Utilities|FlowControl|Switch|SwitchonESlateVisibility _returnvalue_2
    (:Collapsed
      (Class|WidgetBlueprintLibrary|SetFocustoGameViewport))
    (:SelfHitTestInvisible
      (Widget|SetFocus (Variables|Default|GetAs%20CMENU%20SWSelection)))))

(event Custom|OnValueChanged%28Slider02%29
  (params (Vector :type Vector))
  (Transformation|SetActorRelativeRotation (Math|Conversions|RotationFromXVector Vector)))

(event Custom|OnValueChanged%28Slider01%29
  (params (Vector :type Vector))
  (Transformation|SetActorRelativeLocation Vector))

(event Custom|OnNewMessage
  (params (Message :type FSD%20Chat%20Message%20Structure%20%28by%20ref%29))
  (bind _msg (Utilities|IgnoreMsgbySender Message (Variables|Default|GetPlayer%20Character))
    (:CanProceed
      (|Outputs _msg) ; enters at OnReceiveChat
    )))