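; Base actor for shoulder-mounted weapons in a DRG mod, handling ammo, fire cooldown, reloading and muzzle effects.
; Firing plays a montage, decrements the clip and starts timers for cooldown and automatic reload, while automatic weapons re-request fire through ShoulderWeaponSystem.
; Ammo changes, including fractional refills, update a first-person counter widget and fire change notifications.
; Empty reload-start, reload-finished and mag-empty events serve as hooks.
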(event Custom|OnWeaponFired
  (Variables|Default|SetIsReady%28Firerate%29 false)
  (Animation|Montage|PlayMontage (Variables|Default|GetDummyAnimBase) "/Game/_DRGModding/Mod_ShoulderWeaponSystem/Animations/DummyAnim_Fire_Montage.DummyAnim_Fire_Montage"
    (:then
      (bind _result (Math|Integer|DecrementInt (Variables|Default|GetClipSize%28Current%29))
        (:%20%20
          (Default|CallOnClipCountChanged _result)
          (Default|SetClipCount (Variables|Default|GetAs%20Weapon%20Display%20Base%20Ammo%20Count) (Variables|Default|GetClipSize%28Current%29))
          (Utilities|Time|SetTimerbyEvent (delegate Custom|SetCanFire) (Variables|Settings-ShoulderWeapon|GetFireCooldown))
          (if (> (Variables|Default|GetAmmoCount%28Current%29) 0)
            (if (<= (Variables|Default|GetClipSize%28Current%29) 0)
              (Variables|Default|SetIsReloading true)
              (CallFunction|OnReloadStart)
              (Utilities|Time|SetTimerbyEvent (EventDispatchers|CreateEvent :!event Custom|Reload) (Variables|Settings-ShoulderWeapon|GetReloadTime)))
            (else
              (CallFunction|OnMagEmpty))))))))

(event Custom|SetCanFire
  (Variables|Default|SetIsReady%28Firerate%29 true)
  (if (Variables|Settings-ShoulderWeapon|GetIsAutomatic)
    (Default|OnTryWeaponFire (Variables|Default|GetShoulderWeaponSystem))))

(event Custom|OnReloadFinished)

(event Custom|Reload
  (bind _as_weapon_display_base_ammo_count (Variables|Default|GetAs%20Weapon%20Display%20Base%20Ammo%20Count))
  (bind _clipsize_max_ (Variables|Settings-ShoulderWeapon|GetClipSize%28Max%29))
  (Variables|Default|SetIsReloading false)
  (if (< (Variables|Default|GetAmmoCount%28Current%29) (Variables|Settings-ShoulderWeapon|GetClipSize%28Max%29))
    (Variables|Default|SetClipSize%28Current%29 (Variables|Default|GetAmmoCount%28Current%29))
    (Variables|Default|SetAmmoCount%28Current%29 0)
    (else
      (Variables|Default|SetClipSize%28Current%29 _clipsize_max_)
      (Variables|Default|SetAmmoCount%28Current%29 (Math|Integer|Clamp(Integer) (- (Variables|Default|GetAmmoCount%28Current%29) _clipsize_max_) 0 9999))
      (Variables|Default|SetIsReady%28Firerate%29 true)))
  (Default|CallOnClipCountChanged (Variables|Default|GetClipSize%28Current%29))
  (Default|CallOnAmmoCountChanged (Variables|Default|GetAmmoCount%28Current%29))
  (Default|SetClipCount _as_weapon_display_base_ammo_count (Variables|Default|GetClipSize%28Current%29))
  (Default|SetTotalCount _as_weapon_display_base_ammo_count (Variables|Default|GetAmmoCount%28Current%29))
  (Development|PrintString (Utilities|QuickAppend(Macro) (Utilities|String|ToString(Integer) (Variables|Default|GetClipSize%28Current%29)) (Utilities|String|ToString(Integer) (Variables|Default|GetAmmoCount%28Current%29))))
  (CallFunction|OnReloadFinished))

(event Custom|OnReloadStart)

(event Custom|InitializeWeapon
  (Collision|SetActorEnableCollision false)
  (bind _asweapon_display_base_ammo_count (Utilities|Casting|CastToWeaponDisplay_Base_AmmoCount (UserInterface|GetWidget (Variables|Default|GetFirstPersonWidget))))
  (Variables|Default|SetAs%20Weapon%20Display%20Base%20Ammo%20Count _asweapon_display_base_ammo_count)
  (Variables|Default|SetClipSize%28Current%29 (Variables|Settings-ShoulderWeapon|GetClipSize%28Max%29))
  (Variables|Default|SetAmmoCount%28Current%29 (Variables|Settings-ShoulderWeapon|GetAmmoCount%28Max%29))
  (CallFunction|UpdateAmmoCounter))

(event Custom|OnMagEmpty)

(event EventBeginPlay
  (CallFunction|InitializeWeapon))

(fn ConstructionScript)

(fn GetMuzzlePos
  (bind _shoulderweapon (Variables|Default|GetShoulderWeapon))
  (bind _returnvalue (Transformation|GetSocketTransform _shoulderweapon "Muzzle" "RTS_World"))
  (return (.location _returnvalue) (.rotation _returnvalue)))

(fn SpawnMuzzleEffect
  (Class|FirstPersonParticleSystemComponent|SpawnFirstPersonEmitterAttached (Variables|Default|GetEmitter%20Template) (Variables|Default|GetShoulderWeapon) "Muzzle" "0, 0, 0" "0, 0, 0" "1.000000,1.000000,1.000000" "SnapToTarget" true))

(fn PlaySound(Muzzle)
  (params (IsEmpty :type Boolean))
  (Audio|SpawnSoundAttached (select IsEmpty (Variables|Settings-ShoulderWeaponSounds|GetMuzzleSoundEmpty) (Variables|Settings-ShoulderWeaponSounds|GetMuzzleSound)) (Variables|Default|GetShoulderWeapon) "Muzzle" "0, 0, 0" "0, 0, 0" "SnapToTarget" false 1.0 1.0 0.0 0 0))

(fn CanFire
  (return (> (Variables|Default|GetClipSize%28Current%29) 0)))

(fn UpdateAmmoCounter
  (bind _as_weapon_display_base_ammo_count (Variables|Default|GetAs%20Weapon%20Display%20Base%20Ammo%20Count))
  (Default|SetClipCount _as_weapon_display_base_ammo_count (Variables|Default|GetClipSize%28Current%29))
  (Default|SetTotalCount _as_weapon_display_base_ammo_count (Variables|Default|GetAmmoCount%28Current%29)))

(fn Refill
  (params (Amount :type Float%20%28single-precision%29))
  (bind _clipsize_max_ (Variables|Settings-ShoulderWeapon|GetClipSize%28Max%29))
  (bind _ammocount_max_ (Variables|Settings-ShoulderWeapon|GetAmmoCount%28Max%29))
  (if (< (Variables|Default|GetClipSize%28Current%29) (Variables|Settings-ShoulderWeapon|GetClipSize%28Max%29))
    (bind _output_get (Variables|Default|SetClipSize%28Current%29 (select (<= (Math|Integer|Clamp(Integer) (+ (Variables|Default|GetClipSize%28Current%29) (Math|Float|Truncate (* _clipsize_max_ Amount))) 0 _clipsize_max_) 0) 1 (Math|Integer|Clamp(Integer) (+ (Variables|Default|GetClipSize%28Current%29) (Math|Float|Truncate (* _clipsize_max_ Amount))) 0 _clipsize_max_)))))
  (bind _output_get_2 (Variables|Default|SetAmmoCount%28Current%29 (Math|Integer|Clamp(Integer) (+ (Variables|Default|GetAmmoCount%28Current%29) (Math|Float|Truncate (* _ammocount_max_ Amount))) 0 _ammocount_max_)))
  (CallFunction|UpdateAmmoCounter)
  (Default|CallOnClipCountChanged (Variables|Default|GetClipSize%28Current%29))
  (Default|CallOnAmmoCountChanged (Variables|Default|GetAmmoCount%28Current%29))
  (Development|PrintString (Utilities|String|Append (Utilities|String|ToString(Integer) _output_get) " - " (Utilities|String|ToString(Integer) _output_get_2)))
  (Variables|Default|SetIsReady%28Firerate%29 true)
  (Variables|Default|SetIsReloading false))