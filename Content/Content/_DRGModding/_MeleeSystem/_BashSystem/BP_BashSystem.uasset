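; BP_BashSystem adds a weapon bash melee attack for the local player.
; On item equip, it picks a bash type by matching the first-person idle animation, falling back to the item's GetBashMessage for custom types and montages.
; That type's settings load montage, damage, stagger and cooldown, clearing any running cooldown.
; The Bash input plays the montage, damages the target on its notify and starts the cooldown timer.
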(event Custom|OnPlayerCharacterPossesed_Event_0
  (bind _playercharacter (Utilities|GetLocalPlayerCharacter(Macro) true)
    (:Exec
      (bind _output_get (Variables|Default|SetPlayer%20Character _playercharacter))
      (EventDispatchers|BindEventtoOnItemEquipped (Variables|/Script/FSD.PlayerCharacter|GetInventoryComponent _output_get) (delegate Custom|OnItemEquipped))
      (Utilities|FlowControl|DoOnce false
        (:Completed
          (Input|EnableInput (Variables|Default|GetFSDPlayer%20Controller)))))))

(event Custom|OnItemEquipped
  (params (Item :type Item%20Object%20Reference))
  ;[1 1 1] OnItemEquipped - Get if the equipped weapon is bashable or not. If true, do bash related logics.
  (bind _isbashable (CallFunction|PrepareBash (Class|Item|GetCharacterAnimationSet Item)))
  (Variables|Default|SetIs%20Bashable _isbashable))

(event Custom|BashCooldown
  ;[1 1 1] Bash - Play bash animations, does damage when montage notify is executed.
  (Variables|Default|SetIsInCooldown false))

(event EventBeginPlay
  (bind _fsdplayercontroller (Utilities|GetLocalPlayerController(Macro) true)
    (:Completed
      (Variables|Default|SetFSDPlayer%20Controller _fsdplayercontroller)
      (EventDispatchers|AssignOnPlayerCharacterPossesed (Variables|Default|GetFSDPlayer%20Controller) (delegate Custom|OnPlayerCharacterPossesed_Event_0))
      (bind _playercharacter (Utilities|GetLocalPlayerCharacter(Macro) true)
        (:Exec
          (bind _output_get (Variables|Default|SetPlayer%20Character _playercharacter))
          (EventDispatchers|BindEventtoOnItemEquipped (Variables|/Script/FSD.PlayerCharacter|GetInventoryComponent _output_get) (delegate Custom|OnItemEquipped))
          (Utilities|FlowControl|DoOnce false
            (:Completed
              (Input|EnableInput (Variables|Default|GetFSDPlayer%20Controller)))))))))

(event Input|ActionEvents|InputActionBash
  (params (Key :type Key%20Structure :default "None"))
  ;[1 1 1] Bash - Play bash animations, does damage when montage notify is executed.
  (:Pressed
    (if (Variables|Default|GetIs%20Bashable)
      (if (not (Variables|Default|GetIsInCooldown))
        (Animation|Montage|PlayMontage (Variables|/Script/FSD.PlayerCharacter|GetFPMesh (Variables|Default|GetPlayer%20Character)) (Variables|Default|GetMontage%20to%20Play)
          (:then
            (Variables|Default|SetIsInCooldown true)
            (bind _returnvalue (Utilities|Time|SetTimerbyEvent (delegate Custom|BashCooldown) (Variables|Default|GetBash%20Cooldown)))
            (Variables|Default|SetTimer_Cooldown _returnvalue))
          (:OnNotifyBegin
            (Utilities|DamageTarget (Variables|Default|GetPlayer%20Character) 200 (Variables|Default|GetDamage))))))))

(fn ConstructionScript)

(fn PrepareBash
  (params (AnimationSet :type Item%20Character%20Animation%20Set%20Object%20Reference))
  (bind _fp_idle (Variables|/Script/FSD.ItemCharacterAnimationSet|GetFP_Idle AnimationSet))
  (Utilities|IsValid AnimationSet
    (:Is%20Valid
      (Utilities|CompareAnim _fp_idle "/Game/CharacterStructure/Gear_Pistol/FP/FP_Pistol_Idle.FP_Pistol_Idle"
        (:AnimMatch
          (CallFunction|SetStatsbyBashType "NewEnumerator0")
          (return true))
        (:false
          (Utilities|CompareAnim _fp_idle "/Game/CharacterStructure/Gear_Assault/FP/FP_Assault_Idle.FP_Assault_Idle"
            (:AnimMatch
              (CallFunction|SetStatsbyBashType "NewEnumerator1")
              (return true))
            (:false
              (Utilities|CompareAnim _fp_idle "/Game/CharacterStructure/Gear_HeavyLow/FP/FP_Heavy_Idle.FP_Heavy_Idle"
                (:AnimMatch
                  (CallFunction|SetStatsbyBashType "NewEnumerator2")
                  (return true))
                (:false
                  (Utilities|CompareAnim _fp_idle "/Game/CharacterStructure/Gear_DualPistol/FP/FP_ANIM_DualPistol_Idle_A.FP_ANIM_DualPistol_Idle_A"
                    (:AnimMatch
                      (CallFunction|SetStatsbyBashType "NewEnumerator3")
                      (return true))
                    (:false
                      (bind (_isbashable _bashmontage _bashtype) (Class|BPICustomWeaponHandling|GetBash(Message) (Utilities|GetCurrentItem (Variables|Default|GetPlayer%20Character))))
                      (if _isbashable
                        (CallFunction|SetStatsbyBashType _bashtype _bashmontage)
                        (return true)
                        (else
                          (return false))))))))))))
    (:Is%20Not%20Valid
      (return false))))

(fn SetStatsbyBashType
  (params (BashType :type E_BashType%20Enum :default "NewEnumerator0") (CustomBashMontage :type Anim%20Montage%20Object%20Reference))
  (switch Utilities|FlowControl|Switch|SwitchonE_BashType BashType
    (:NewEnumerator0
      (CallFunction|SetStats "/Game/_DRGModding/_MeleeSystem/_BashSystem/BashSetting_Pistol.BashSetting_Pistol" CustomBashMontage))
    (:NewEnumerator1
      (CallFunction|SetStats "/Game/_DRGModding/_MeleeSystem/_BashSystem/BashSetting_Rifle.BashSetting_Rifle" CustomBashMontage))
    (:NewEnumerator2
      (CallFunction|SetStats "/Game/_DRGModding/_MeleeSystem/_BashSystem/BashSetting_Heavy.BashSetting_Heavy" CustomBashMontage))
    (:NewEnumerator3
      (CallFunction|SetStats "/Game/_DRGModding/_MeleeSystem/_BashSystem/BashSetting_DualPistol.BashSetting_DualPistol" CustomBashMontage))))

(fn SetStats
  (params (Target :type Bash%20Settings%20Object%20Reference) (CustomBashMontage :type Anim%20Montage%20Object%20Reference))
  (Utilities|IsValid CustomBashMontage
    (:Is%20Valid
      (Variables|Default|SetMontage%20to%20Play CustomBashMontage))
    (:Is%20Not%20Valid
      (Variables|Default|SetMontage%20to%20Play (Variables|/Game/_DRGModding/_MeleeSystem/_BashSystem/BashSettings.BashSettings_C|GetBashMontage Target))))
  (Variables|/Script/FSD.DamageComponent|SetDamage (Variables|Default|GetDamage) (Variables|/Game/_DRGModding/_MeleeSystem/_BashSystem/BashSettings.BashSettings_C|GetDamage Target))
  (Variables|/Script/FSD.DamageComponent|SetStaggerOnlyOnWeakpointHit (Variables|Default|GetDamage) (Variables|/Game/_DRGModding/_MeleeSystem/_BashSystem/BashSettings.BashSettings_C|GetWeakPointOnly Target))
  (Variables|/Script/FSD.DamageComponent|SetStaggerChance (Variables|Default|GetDamage) (Variables|/Game/_DRGModding/_MeleeSystem/_BashSystem/BashSettings.BashSettings_C|GetStunChange Target))
  (Variables|/Script/FSD.DamageComponent|SetStaggerDuration (Variables|Default|GetDamage) (Variables|/Game/_DRGModding/_MeleeSystem/_BashSystem/BashSettings.BashSettings_C|GetStunDuration Target))
  (Variables|Default|SetBash%20Cooldown (Variables|/Game/_DRGModding/_MeleeSystem/_BashSystem/BashSettings.BashSettings_C|GetBashCooldown Target))
  (Utilities|Time|ClearandInvalidateTimerbyHandle (Variables|Default|GetTimer_Cooldown))
  (Variables|Default|SetIsInCooldown false))