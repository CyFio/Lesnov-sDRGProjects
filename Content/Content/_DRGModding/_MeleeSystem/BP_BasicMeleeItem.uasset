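; BP_BasicMeleeItem is a base melee item for a Deep Rock Galactic modding melee system, providing shared setup and input hooks.
; On BeginPlay it caches the local player controller and character.
; When UseInput is set, equipping and unequipping toggle input on that controller, forwarding Cycleitem press and release to empty events for overriding.
; A DebugMessage helper prints prefixed text to chat, controlled by DisableDebug.
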(event Custom|OnCycleItemPressed)

(event Custom|OnCycleItemReleased)

(event EventBeginPlay
  (bind _fsdplayercontroller (Utilities|GetLocalPlayerController(Macro) true)
    (:Completed
      (Variables|Default|SetFSDPlayer%20Controller _fsdplayercontroller)
      (bind _playercharacter (Utilities|GetLocalPlayerCharacter(Macro) true)
        (:Exec
          (Variables|Default|SetPlayer%20Character _playercharacter))))))

(event EventRecieveEquipped
  (if (Variables|BasicMeleeItem-Settings|GetUseInput)
    (Input|EnableInput (Variables|Default|GetFSDPlayer%20Controller))))

(event EventRecieveUnequipped
  (if (Variables|BasicMeleeItem-Settings|GetUseInput)
    (Input|DisableInput (Variables|Default|GetFSDPlayer%20Controller))))

(event Input|ActionEvents|InputActionCycleitem
  (params (Key :type Key%20Structure :default "None"))
  (:Pressed
    (CallFunction|OnCycleItemPressed))
  (:Released
    (CallFunction|OnCycleItemReleased)))

(fn ConstructionScript)

(fn DebugMessage
  (params (Sender :type String) (Text :type String))
  (Utilities|PrintViaChat (Variables|Default|GetDisable%20Debug) (Utilities|QuickAppend(Macro) (Variables|Settings-Debug|GetDebugName) Sender) Text "NormalUser"))